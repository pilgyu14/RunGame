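; Runner character Blueprint that adds a slide move on Left Shift.
; The slide shrinks the capsule, plays a montage, then restores capsule height after a fixed delay, with a DoOnce blocking re-entry until then.
; The mesh shifts along world negative X at both start and end, so the offset is never undone.
; The speed check is ANDed with false and only feeds DoOnce's start state, so it never gates the slide.
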(event `self.CapsuleComponent.OnComponentBeginOverlap`
  (params (OverlappedComponent :type "PrimitiveComponent Object Reference") (OtherActor :type "Actor Object Reference") (OtherComp :type "PrimitiveComponent Object Reference") (OtherBodyIndex :type Integer) (bFromSweep :type Boolean) (SweepResult :type "HitResult Structure (by ref)")))

(event `Key|LeftShift`
  (params (Key :type "Key Structure"))
  (:`Pressed`
    (if true
      (`/Engine/EditorBlueprintResources/StandardMacros.DoOnce` (and (> (`KismetMathLibrary.VSize` (`MovementComponent.Velocity` (`self.CharacterMovement`))) 10.0) false) :!label _label
        (:`Completed`
          (`CapsuleComponent.SetCapsuleHalfHeight` (`self.CapsuleComponent`) 28.0 true)
          (`SceneComponent.K2_SetWorldLocation` (`self.Mesh`) (+ (`SceneComponent.K2_GetComponentLocation` (`self.Mesh`)) (-5.0 0.0 0.0)) false false)
          (`self.PlayAnimMontage` "/Game/Animations/SlideAnimMontage.SlideAnimMontage")
          (`KismetSystemLibrary.Delay` 0.8)
          (`CapsuleComponent.SetCapsuleHalfHeight` (`self.CapsuleComponent`) 96.0 true)
          (`SceneComponent.K2_SetWorldLocation` (`self.Mesh`) (+ (`SceneComponent.K2_GetComponentLocation` (`self.Mesh`)) (-5.0 0.0 0.0)) false false)
          (goto _label :!via `Reset`))))))

(fn `UserConstructionScript`)